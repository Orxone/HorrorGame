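; BP_Door is a lockable door actor that swings open and closed on interaction when HasKey is true, and otherwise prints that a key is needed.
; OnInteract toggles IsClosed, plays the lock sound and runs the Open timeline forward or in reverse, lerping the Pivot's yaw between 0 and -90 degrees.
; The PickUpKey event sets HasKey to false, despite its name suggesting the opposite.
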(event EventBeginPlay
  (|CallParentFunction) ; This node is disabled and will not be called.\nDrag off pins to build functionality.
)

(event Collision|EventActorBeginOverlap
  (params (OtherActor :type Actor%20Object%20Reference))
  (|CallParentFunction OtherActor) ; This node is disabled and will not be called.\nDrag off pins to build functionality.
)

(event EventTick
  (params (DeltaSeconds :type Float%20%28single-precision%29))
  (|CallParentFunction DeltaSeconds) ; This node is disabled and will not be called.\nDrag off pins to build functionality.
)

(event EventOnInteract
  (params (Interacting%20Play :type Character%20Object%20Reference))
  (if (Variables|Default|GetHasKey?)
    (if (Variables|Default|GetIsClosed)
      (Variables|Default|SetIsClosed false)
      (Audio|PlaySound2D "/Game/Audio/Sounds/LockOpening.LockOpening" 1.0 1.0 0.0 0 0)
      (bind _alpha (Timeline|Open Play)
        (:Update
          (Transformation|SetRelativeRotation (Variables|Default|GetPivot) (Math|Rotator|MakeRotator 0.0 0.0 (Math|Float|Lerp 0.0 -9e+01 _alpha)) false false)))
      (else
        (Variables|Default|SetIsClosed true)
        (Audio|PlaySound2D "/Game/Audio/Sounds/LockOpening.LockOpening" 1.0 1.0 0.0 0 0)
        (Timeline|Open Reverse)))
    (else
      (Development|PrintString "You need a key" true true "(R=1.000000,G=0.000000,B=0.058054,A=1.000000)"))))

(event EventPickUpKey
  (Variables|Default|SetHasKey? false))

(fn ConstructionScript
  (|CallParentFunction))