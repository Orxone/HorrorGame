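; BP_Notes is an interactable note actor that the player can read.
; On interact, it copies its note description to the player, sets the reading flag, plays a page sound and has the player show the note.
; When an overlap with its collision component ends, it hides the note and clears the reading flag.
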(event OnComponentEndOverlap(Collision)
  (params (OverlappedComponent :type Primitive%20Component%20Object%20Reference) (OtherActor :type Actor%20Object%20Reference) (OtherComp :type Primitive%20Component%20Object%20Reference) (OtherBodyIndex :type Integer))
  ;[1 1 1] Hide
  (Default|HideNote (Variables|Default|GetPlayer%20Ref))
  (Variables|/Game/Blueprints/BP_Player.BP_Player_C|SetIsReading? (Variables|Default|GetPlayer%20Ref) false))

(event EventBeginPlay
  (|CallParentFunction) ; This node is disabled and will not be called.\nDrag off pins to build functionality.
)

(event Collision|EventActorBeginOverlap
  (params (OtherActor :type Actor%20Object%20Reference))
  (|CallParentFunction OtherActor) ; This node is disabled and will not be called.\nDrag off pins to build functionality.
)

(event EventTick
  (params (DeltaSeconds :type Float%20%28single-precision%29))
  (|CallParentFunction DeltaSeconds) ; This node is disabled and will not be called.\nDrag off pins to build functionality.
)

(event EventOnInteract
  (params (Interacting%20Play :type Character%20Object%20Reference))
  (Variables|/Game/Blueprints/BP_Player.BP_Player_C|SetNote (Variables|Default|GetPlayer%20Ref) (Variables|Default|GetNoteDescription))
  (Variables|/Game/Blueprints/BP_Player.BP_Player_C|SetIsReading? (Variables|Default|GetPlayer%20Ref) true)
  (Audio|PlaySound2D "/Game/Audio/Sounds/Page_Cue.Page_Cue" 1.0 1.0 0.0 0 0)
  (Default|ShowNote (Variables|Default|GetPlayer%20Ref)))

(fn ConstructionScript
  (|CallParentFunction))

(fn IsInteractable
  (return true))