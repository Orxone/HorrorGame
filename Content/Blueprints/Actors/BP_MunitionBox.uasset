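; BP_MunitionBox is an interactable ammo box actor that is picked up on interaction.
; OnInteract plays a heavy opening sound, sends PickUpAmmoMessage through MunitionBox, prints a pickup message and destroys the actor.
; A separate OpenBox event toggles IsClosed and plays or reverses a timeline that lerps MunitionBox's relative yaw to swing it open or shut.
; IsInteractable always returns true.
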(event Custom|OpenBox
  ;[1 1 1] BoxOpenAnimation
  (if (Variables|Default|GetIsClosed)
    (Variables|Default|SetIsClosed false)
    (bind _alpha (Timeline|BoxOpening Play)
      (:Update
        (Transformation|SetRelativeRotation (Variables|Default|GetMunitionBox) (Math|Rotator|MakeRotator 0.0 0.0 (Math|Float|Lerp 0.0 -9e+01 _alpha)) false false)))
    (else
      (Variables|Default|SetIsClosed true)
      (Timeline|BoxOpening Reverse))))

(event EventBeginPlay)

(event Collision|EventActorBeginOverlap
  (params (OtherActor :type Actor%20Object%20Reference)))

(event EventTick
  (params (DeltaSeconds :type Float%20%28single-precision%29)))

(event EventOnInteract
  (params (Interacting%20Play :type Character%20Object%20Reference))
  ;[1 1 1] Interact
  (Audio|PlaySound2D "/Game/Audio/Sounds/HeavyOpening.HeavyOpening" 1.0 1.0 0.0 0 0)
  (Class|BPIPickUpAmmo|PickUpAmmo(Message) (Variables|Default|GetMunitionBox))
  (Development|PrintString "You got ammo")
  (Actor|DestroyActor))

(fn ConstructionScript)

(fn IsInteractable
  (return true))