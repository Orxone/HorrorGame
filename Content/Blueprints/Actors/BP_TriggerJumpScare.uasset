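; BP_TriggerJumpScare is a trigger actor that fires a one-time jump scare on the player.
; On BeginPlay it caches the player character as BP_Player.
; The first Box begin overlap calls JUMPSCARE on that player after a one-second delay, and the first end overlap calls JUMPSCAREOFF immediately.
; Separate DoOnce gates keep each call from repeating, and neither overlap checks which actor triggered it.
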(event OnComponentBeginOverlap(Box)
  (params (OverlappedComponent :type Primitive%20Component%20Object%20Reference) (OtherActor :type Actor%20Object%20Reference) (OtherComp :type Primitive%20Component%20Object%20Reference) (OtherBodyIndex :type Integer) (bFromSweep :type Boolean) (SweepResult :type Hit%20Result%20Structure%20%28by%20ref%29))
  (Utilities|FlowControl|DoOnce false
    (:Completed
      (Utilities|FlowControl|Delay 1.0)
      (Default|JUMPSCARE (Variables|Default|GetBP%20Player%20ref)))))

(event OnComponentEndOverlap(Box)
  (params (OverlappedComponent :type Primitive%20Component%20Object%20Reference) (OtherActor :type Actor%20Object%20Reference) (OtherComp :type Primitive%20Component%20Object%20Reference) (OtherBodyIndex :type Integer))
  (Utilities|FlowControl|DoOnce false
    (:Completed
      (Default|JUMPSCAREOFF (Variables|Default|GetBP%20Player%20ref)))))

(event EventBeginPlay
  (bind _asbp_player (Utilities|Casting|CastToBP_Player (Game|GetPlayerCharacter 0)))
  (Variables|Default|SetBP%20Player%20ref _asbp_player))

(event Collision|EventActorBeginOverlap
  (params (OtherActor :type Actor%20Object%20Reference)))

(event EventTick
  (params (DeltaSeconds :type Float%20%28single-precision%29)))

(fn ConstructionScript)