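; BP_Medikit is an interactable health pickup that is consumed when the player uses it.
; OnInteract casts the interactor to BP_Player, plays a sound, and shows pickup messages through the Medikit reference and a debug print.
; It then passes the player's health plus a fixed bonus, clamped to the valid range, to UpdateHealthBar and destroys itself.
; IsInteractable always returns true.
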(event EventBeginPlay)

(event EventTick
  (params (DeltaSeconds :type Float%20%28single-precision%29)))

(event EventOnInteract
  (params (Interacting%20Play :type Character%20Object%20Reference))
  ;[1 1 1] Interact
  (bind _asbp_player (Utilities|Casting|CastToBP_Player Interacting%20Play))
  (Audio|PlaySound2D "/Game/Audio/Sounds/HeavyOpening.HeavyOpening" 1.0 1.0 0.0 0 0)
  (Class|BPIPickUpMedikit|PickUpMedikit(Message) (Variables|Default|GetMedikit))
  (Development|PrintString "You got a medikit")
  (Default|UpdateHealthBar _asbp_player (Math|Float|Clamp(Float) (+ (Variables|/Game/Blueprints/Characters/Player/BP_Player.BP_Player_C|GetHealth _asbp_player) 15.0) 0.0 1e+02) false)
  (Actor|DestroyActor))

(fn ConstructionScript)

(fn IsInteractable
  (return true))