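; BP_BearTrap is a trap actor that catches BP_Player on overlap and holds them until they mash R to escape.
; Catching disables movement, snaps the player to the trap's horizontal centre, plays a sound, enables input and switches off the box collision.
; Enough R presses restore walking, then collision re-arms after a delay.
; A retriggerable delay on key release resets the press count when mashing pauses.
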(event OnComponentBeginOverlap(BoxCollision)
  (params (OverlappedComponent :type Primitive%20Component%20Object%20Reference) (OtherActor :type Actor%20Object%20Reference) (OtherComp :type Primitive%20Component%20Object%20Reference) (OtherBodyIndex :type Integer) (bFromSweep :type Boolean) (SweepResult :type Hit%20Result%20Structure%20%28by%20ref%29))
  (bind _asbp_player (Utilities|Casting|CastToBP_Player OtherActor))
  (CallFunction|CatchPlayer _asbp_player)
  (Input|EnableInput (Game|GetPlayerController 0) 0)
  (Collision|SetCollisionEnabled (Variables|Default|GetBox%20Collision) "NoCollision"))

(event Custom|Catch%20Player
  (params (Player :type Character%20Object%20Reference))
  (bind _box_collision (Variables|Default|GetBox%20Collision))
  (bind _returnvalue (Transformation|GetWorldLocation _box_collision))
  (Pawn|Components|CharacterMovement|DisableMovement (Variables|/Script/Engine.Character|GetCharacterMovement Player))
  (Transformation|SetActorLocation Player (Math|Vector|MakeVector (.x _returnvalue) (.y _returnvalue) (.z (Transformation|GetActorLocation Player))) false false)
  (Audio|PlaySound2D "/Game/Audio/Sounds/Bear_Trap_Cue.Bear_Trap_Cue" 1.0 1.0 0.0 0 0))

(event Custom|OpenTrap
  ;[1 1 1] Open and retrigger
  (Pawn|Components|CharacterMovement|SetMovementMode (Variables|/Script/Engine.Character|GetCharacterMovement (stale OnComponentBeginOverlap(BoxCollision) _asbp_player)) "MOVE_Walking" 0)
  (Utilities|FlowControl|Delay 3.0)
  (Collision|SetCollisionEnabled (Variables|Default|GetBox%20Collision) "QueryAndPhysics"))

(event Input|KeyboardEvents|R
  (params (Key :type Key%20Structure :default "None"))
  (:Pressed
    (bind _result (Math|Integer|IncrementInt (Variables|Presses|GetPresses))
      (:%20%20
        (if (== _result (Variables|Presses|GetPresses%20Required))
          (CallFunction|OpenTrap)))))
  (:Released
    (Utilities|FlowControl|RetriggerableDelay 0.5)
    (Variables|Presses|SetPresses 0)))

(fn ConstructionScript)