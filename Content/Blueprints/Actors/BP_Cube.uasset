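; BP_Cube is an interactable collectible cube that counts toward the player's victory.
; On interact it plays a sound, calls its pickup message, increments the player's CPickups, then destroys itself and spawns a BP_Obsidian at its location.
; It calls VictoryTrigger on the cached BP_Player once the count reaches six.
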(event EventBeginPlay
  (bind _asbp_player (Utilities|Casting|CastToBP_Player (Game|GetPlayerCharacter 0)))
  (Variables|Default|SetPlayer%20Ref _asbp_player))

(event Collision|EventActorBeginOverlap
  (params (OtherActor :type Actor%20Object%20Reference)))

(event EventTick
  (params (DeltaSeconds :type Float%20%28single-precision%29)))

(event EventOnInteract
  (params (Interacting%20Play :type Character%20Object%20Reference))
  (bind _player_ref (Variables|Default|GetPlayer%20Ref))
  (Audio|PlaySound2D "/Game/Audio/Sounds/CubeSound_Cue.CubeSound_Cue" 1.0 1.0 0.0 0 0)
  (Class|BPIPickUCubes|PickUpCube(Message) (Variables|Default|GetCube))
  (Variables|/Game/Blueprints/Characters/Player/BP_Player.BP_Player_C|SetCPickups _player_ref (+ (Variables|/Game/Blueprints/Characters/Player/BP_Player.BP_Player_C|GetCPickups _player_ref) 1))
  (bind _output_get (Variables|Default|SetCubeLocation (Transformation|GetActorLocation)))
  (Actor|DestroyActor)
  (Game|SpawnActorfromClass "/Game/Blueprints/Actors/BP_Obsidian.BP_Obsidian_C" (Math|Transform|MakeTransform _output_get "0, 0, 0" "1.000000,1.000000,1.000000") "Undefined" "MultiplyWithRoot" 0 0)
  (if (>= (Variables|/Game/Blueprints/Characters/Player/BP_Player.BP_Player_C|GetCPickups _player_ref) 6)
    (Default|VictoryTrigger _player_ref)))

(fn ConstructionScript)

(fn IsInteractable
  (return true))